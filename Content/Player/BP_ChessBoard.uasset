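; Checkers board actor that spawns an 8x8 grid of square and piece meshes at BeginPlay, tracked in index-based arrays.
; ClickReplicationServer feeds Click, which maps world positions to indices, highlighting the first click and computing diagonal steps per color.
; The second click moves the piece or captures the opposing one at the midpoint index.
; When either color runs out, it pauses the game and shows the GameOver widget.
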(event `self.ReceiveBeginPlay`
  (for _index (range 64)
    (`|ExecutionSequence`
      (:`then_0`
        ;[1 1 1] Установка игр поля
        (bind _returnvalue (`AddComponent|NODE_AddStaticMeshComponent-10` :`RelativeTransform` (`KismetMathLibrary.Conv_VectorToTransform` (`self.IndexToPosition` _index))))
        (`KismetArrayLibrary.Array_Add` (`self.Fieds_Mesh`) _returnvalue)
        (bind _returnvalue_2 (select `bool` (xor (`KismetMathLibrary.Conv_IntToBool` (mod _index 2)) (`KismetMathLibrary.Conv_IntToBool` (mod (/ _index 8) 2))) :`false` "/Game/Assets/Materials/BoardBlack.BoardBlack" :`true` "/Game/Assets/Materials/BoardWhite.BoardWhite" :!type "Material Object Reference"))
        (`PrimitiveComponent.SetMaterial` _returnvalue 0 _returnvalue_2)
        (`KismetArrayLibrary.Array_Add` (`self.Fields_Material`) _returnvalue_2))
      (:`then_1`
        ;[1 1 1] Установка шашек
        (bind _returnvalue_3 (`AddComponent|NODE_AddStaticMeshComponent-18` :`RelativeTransform` (`KismetMathLibrary.MakeTransform` (`self.IndexToPosition200` _index) (struct :`Roll` 90.0) (3.0 2.0 3.0))))
        (bind _output (`|GetArrayItem` (`self.Start_Figure`) _index))
        (`StaticMeshComponent.SetStaticMesh` _returnvalue_3 (select `int` _output :`0` null :`1` (select `int` (`KismetMathLibrary.Conv_BoolToInt` (> 30 _index)) :`0` "/Game/Assets/CheckerBlack.CheckerBlack" :`1` "/Game/Assets/CheckerWhite.CheckerWhite" :!type "StaticMesh Object Reference")))
        (`KismetArrayLibrary.Array_Add` (`self.Piecies_Mesh`) _returnvalue_3)
        (`KismetArrayLibrary.Array_Add` (`self.NoEmptyFields`) (`KismetMathLibrary.Conv_IntToBool` _output))))))

(event `ClickReplicationClient`
  (params (Position :type "Vector Structure")))

(event `ClickReplicationServer`
  (params (Position :type "Vector Structure"))
  (`self.Click` Position))

(fn `Click`
  (params (Position :type "Vector Structure"))
  (locals (IndexCanMoveWhite :type "Array of Integer") (IndexCanMoveBlack :type "Array of Integer"))
  (bind _returnvalue (`self.PositionToIndex` Position))
  (bind _canmovewhite (`self.CanMoveWhite`))
  (bind _canmoveblack (`self.CanMoveBlack`))
  (bind _returnvalue_2 (/ (+ (`self.FirstClick`) (`self.SecondClick`)) 2))
  (bind _output (`|GetArrayItem` (`self.Piecies_Mesh`) _returnvalue_2))
  (bind _staticmesh (`StaticMeshComponent.StaticMesh` _output))
  (if (== (`self.FirstClick`) -1)
    (`PrimitiveComponent.SetMaterial` (`|GetArrayItem` (`self.Fieds_Mesh`) _returnvalue) 0 "/Game/Assets/Materials/BoardActiv.BoardActiv")
    (bind _output_get (set `self.FirstClick` _returnvalue))
    (bind _returnvalue_3 (+ _output_get -7))
    (bind _returnvalue_4 (/ _output_get 8))
    (bind _returnvalue_5 (- _returnvalue_4 1))
    ;[1 1 1] Определение возможных ходов
    (if (== (/ _returnvalue_3 8) _returnvalue_5)
      (`KismetArrayLibrary.Array_Add` _canmoveblack _returnvalue_3))
    (bind _returnvalue_6 (+ _output_get -9))
    (if (== (/ _returnvalue_6 8) _returnvalue_5)
      (`KismetArrayLibrary.Array_Add` _canmoveblack _returnvalue_6))
    (bind _returnvalue_7 (+ _output_get 7))
    (bind _returnvalue_8 (+ _returnvalue_4 1))
    (if (== (/ _returnvalue_7 8) _returnvalue_8)
      (`KismetArrayLibrary.Array_Add` _canmovewhite _returnvalue_7))
    (bind _returnvalue_9 (+ _output_get 9))
    (if (== (/ _returnvalue_9 8) _returnvalue_8)
      (`KismetArrayLibrary.Array_Add` _canmovewhite _returnvalue_9))
    (else
      (bind _output_get_2 (set `self.SecondClick` _returnvalue))
      (if (not (`|GetArrayItem` (`self.NoEmptyFields`) _output_get_2))
        ;[1 1 1] Ход по правилам
        (if (== (`StaticMeshComponent.StaticMesh` (`|GetArrayItem` (`self.Piecies_Mesh`) (`self.FirstClick`))) "/Game/Assets/CheckerWhite.CheckerWhite")
          (if (`KismetArrayLibrary.Array_Contains` (`self.CanMoveWhite`) _output_get_2)
            (`self.SetMaterial` :!label _label)
            (`self.MoveStep`)
            (else
              (`self.SetMaterial` :!label _label_2)
              (if (== (`|GetArrayItem` (`self.Fields_Material`) (`self.SecondClick`)) "/Game/Assets/Materials/BoardBlack.BoardBlack")
                (`/Engine/EditorBlueprintResources/StandardMacros.IsValid` _staticmesh
                  (:`Is Valid`
                    (if (!= (`StaticMeshComponent.StaticMesh` (`|GetArrayItem` (`self.Piecies_Mesh`) (`self.FirstClick`))) _staticmesh)
                      (`self.MoveStep`)
                      (if true
                        (if (== _staticmesh "/Game/Assets/CheckerWhite.CheckerWhite")
                          (bind _output_get_3 (set `self.AmountWhite` (- (`self.AmountWhite`) 1)))
                          (else
                            (bind _output_get_4 (set `self.AmountBlack` (- (`self.AmountBlack`) 1)))))
                        (`ActorComponent.K2_DestroyComponent` _output)
                        (`KismetArrayLibrary.Array_Set` (`self.NoEmptyFields`) _returnvalue_2)
                        (bind _returnvalue_10 (< _output_get_3 1))
                        (if (xor _returnvalue_10 (< _output_get_4 1))
                          (set `self.WinnerWhite` (not _returnvalue_10))
                          ;[1 1 1] Окончание игры + виджет GameOver
                          (`GameplayStatics.SetGamePaused` true)
                          (`/Engine/EditorBlueprintResources/StandardMacros.IsValid` (`self.GameOver_W`)
                            (:`Is Valid`
                              _)
                            (:`Is Not Valid`
                              (bind _returnvalue_11 (`|CreateWidget` "/Game/UI/AllLevels/GameOver.GameOver_C"))
                              (set `self.GameOver_W` _returnvalue_11)
                              (set `/Game/UI/AllLevels/GameOver.GetWinner` self _returnvalue_11)))
                          (`UserWidget.AddToViewport` (`self.GameOver_W`) 0)
                          (return)
                          (else
                            _)))))
                  (:`Is Not Valid`
                    _)))))
          (elif (`KismetArrayLibrary.Array_Contains` (`self.CanMoveBlack`) _output_get_2)
            (goto _label)
            (else
              (goto _label_2))))
        (else
          (goto _label_2)))
      (set `self.FirstClick` -1)
      (`KismetArrayLibrary.Array_Clear` (`self.CanMoveWhite`))
      (`KismetArrayLibrary.Array_Clear` (`self.CanMoveBlack`)))))

(fn `MoveStep`
  (bind _secondclick (`self.SecondClick`))
  (bind _output (`|GetArrayItem` (`self.Piecies_Mesh`) (`self.FirstClick`)))
  (`SceneComponent.K2_SetWorldLocation` _output (`self.IndexToPosition200` (`self.SecondClick`)) false false)
  (`KismetArrayLibrary.Array_Set` (`self.Piecies_Mesh`) _secondclick _output)
  (`KismetArrayLibrary.Array_Set` (`self.NoEmptyFields`) (`self.FirstClick`))
  (`KismetArrayLibrary.Array_Set` (`self.NoEmptyFields`) _secondclick true)
  (return))

(fn `OnRep_Piecies_Mesh`)

(fn `UserConstructionScript`)