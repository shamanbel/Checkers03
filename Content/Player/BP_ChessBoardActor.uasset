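; Checkers board actor that builds an 8x8 field and handles piece movement by clicks.
; BeginPlay adds alternately colored square meshes and spawns two colors of BP_Pawn from the StartFigure layout.
; A server click event feeds Click, which highlights the first square, then moves its piece to the second.
; Index jumps of 14 or more destroy the midpoint piece; no move legality checks run, and the client event and OnRep are empty.
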(event Custom|ClickReplicationServer
  (params (Position :type Vector))
  (CallFunction|Click Position))

(event Custom|ClickReplicationClient
  (params (Position :type Vector)))

(event EventBeginPlay
  (for _index (range 0 63)
    (Utilities|FlowControl|Sequence
      (:then_0
        (bind _returnvalue (AddComponent|AddStaticMeshComponent false (Math|Conversions|ToTransform(Vector) (Utilities|IndextoPosition _index))))
        (Utilities|Array|Add (Variables|Default|GetFieds_Mesh) _returnvalue)
        (Rendering|Material|SetMaterial _returnvalue 0 (select (Class|KismetMathLibrary|XORBoolean (Math|Conversions|ToBoolean(Integer) (Math|Integer|%(Integer) _index 2)) (Math|Conversions|ToBoolean(Integer) (Math|Integer|%(Integer) (/ _index 8) 2))) "/Game/Assets/Materials/BoardWhite.BoardWhite" "/Game/Assets/Materials/BoardBlack.BoardBlack"))
        (Utilities|Array|Add (Variables|Default|GetFields_Material) (select (Class|KismetMathLibrary|XORBoolean (Math|Conversions|ToBoolean(Integer) (Math|Integer|%(Integer) _index 2)) (Math|Conversions|ToBoolean(Integer) (Math|Integer|%(Integer) (/ _index 8) 2))) "/Game/Assets/Materials/BoardWhite.BoardWhite" "/Game/Assets/Materials/BoardBlack.BoardBlack")))
      (:then_1
        (if (Math|Conversions|ToBoolean(Integer) (Utilities|Array|Get(acopy) (Variables|Default|GetStart_Figure) _index))
          (bind _returnvalue_2 (Game|SpawnActorfromClass "/Game/Player/BP_Pawn.BP_Pawn_C" (Math|Transform|MakeTransform (Utilities|IndextoPosition200 _index) "0, 0,90.000000" "3.000000,2.000000,3.000000") "Undefined" 0 0))
          (Rendering|Material|SetMaterial (Variables|/Game/Player/BP_Pawn.BP_Pawn_C|GetStaticMesh _returnvalue_2) 0 (Utilities|Select :Index (Math|Conversions|ToInteger(Boolean) (> 30 _index)) :Option%200 "/Game/Assets/Materials/CheckerColor01.CheckerColor01" :Option%201 "/Game/Assets/Materials/CheckerColor02.CheckerColor02")))
        (Utilities|Array|Add (Variables|Default|GetPiecies_Mesh) (Utilities|Select :Index (Utilities|Array|Get(acopy) (Variables|Default|GetStart_Figure) _index) :Option%200 0 :Option%201 _returnvalue_2))))))

(fn ConstructionScript)

(fn Click
  (params (Position :type Vector))
  (if (== (Variables|Default|GetFirstClick) -1)
    (Rendering|Material|SetMaterial (Utilities|Array|Get(acopy) (Variables|Default|GetFieds_Mesh) (stale _returnvalue)) 0 "/Game/Assets/Materials/BoardActiv.BoardActiv")
    (Variables|Default|SetFirstClick (stale _returnvalue))
    (else
      (bind _output_get (Variables|Default|SetSecondClick (stale _returnvalue)))
      (Rendering|Material|SetMaterial (Utilities|Array|Get(acopy) (Variables|Default|GetFieds_Mesh) (Variables|Default|GetFirstClick)) 0 (Utilities|Array|Get(acopy) (Variables|Default|GetFields_Material) (Variables|Default|GetFirstClick)))
      (Transformation|SetActorLocation (Utilities|Array|Get(acopy) (Variables|Default|GetPiecies_Mesh) (Variables|Default|GetFirstClick)) (Utilities|IndextoPosition200 _output_get) false false)
      (Utilities|Array|SetArrayElem (Variables|Default|GetPiecies_Mesh) _output_get (Utilities|Array|Get(acopy) (Variables|Default|GetPiecies_Mesh) (Variables|Default|GetFirstClick)))
      (if (Class|KismetMathLibrary|XORBoolean (>= (- (Variables|Default|GetSecondClick) (Variables|Default|GetFirstClick)) 14) (<= (- (Variables|Default|GetSecondClick) (Variables|Default|GetFirstClick)) -14))
        (Actor|DestroyActor (Utilities|Array|Get(acopy) (Variables|Default|GetPiecies_Mesh) (/ (+ (Variables|Default|GetFirstClick) _output_get) 2)))
        (else
          (Variables|Default|SetFirstClick -1))))))

(fn OnRepPieciesMesh)